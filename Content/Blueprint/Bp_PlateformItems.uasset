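; Item platform that spawns a configured actor class when the actor referenced by RefMaster leaves its Box volume.
; The construction script shows PreviewMesh on the Preview component.
; On a matching end overlap, SpawnActor spawns at the Arrow's location and rotation with reduced scale, then clears RefMaster, which this graph never otherwise assigns.
; BeginPlay caches the first-person character, and a debug "Hello" prints after spawning.
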(event OnComponentEndOverlap(Box)
  (params (OverlappedComponent :type Primitive%20Component%20Object%20Reference) (OtherActor :type Actor%20Object%20Reference) (OtherComp :type Primitive%20Component%20Object%20Reference) (OtherBodyIndex :type Integer))
  (if (== OtherActor (Variables|Default|GetRefMaster))
    (CallFunction|SpawnActor (Variables|Default|GetActorSpawn))
    (Development|PrintString "Hello")))

(event EventBeginPlay
  (bind _asbp_first_person_character (Utilities|Casting|CastToBP_FirstPersonCharacter (Game|GetPlayerCharacter 0)))
  (Variables|Default|SetAs%20BP%20First%20Person%20Character _asbp_first_person_character))

(fn ConstructionScript
  (Components|StaticMesh|SetStaticMesh (Variables|Default|GetPreview) (Variables|Mesh|GetPreviewMesh)))

(fn SpawnActor
  (params (Class :type Actor%20Class%20Reference))
  (bind _arrow (Variables|Default|GetArrow))
  (bind _returnvalue (Transformation|GetWorldTransform _arrow))
  (Game|SpawnActorfromClass Class (Math|Transform|MakeTransform (.location _returnvalue) (.rotation _returnvalue) "0.800000,0.800000,0.800000") "Undefined" 0 0)
  (Variables|Default|SetRefMaster 0))