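; Master_Object is a physics object that the first-person character can grab and release.
; Grabbing attaches it to the character's GrabLocation, and Tick lerps its transform toward that point while held.
; Releasing detaches it in world space and turns physics simulation back on.
; Every tick also clamps its linear velocity to MaxVelocity.
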(event EventTick
  (params (DeltaSeconds :type Float%20%28single-precision%29))
  (CallFunction|UpdateVelocity)
  (if (Variables|Default|GetGrab?)
    (CallFunction|InterpolateGrabbing (Utilities|Time|GetWorldDeltaSeconds) 5.0)))

(event EventGrabbing
  (Variables|Default|SetGrab? true)
  (CallFunction|Grab))

(event EventBeginPlay
  (bind _asbp_first_person_character (Utilities|Casting|CastToBP_FirstPersonCharacter (Game|GetPlayerCharacter 0)))
  (Variables|Default|SetAs%20BP%20First%20Person%20Character _asbp_first_person_character))

(event EventUngrabbe
  (Variables|Default|SetGrab? false)
  (CallFunction|Ungrab))

(fn ConstructionScript)

(fn UpdateVelocity
  (bind _maxvelocity (Variables|Default|GetMaxVelocity))
  (bind _returnvalue (Physics|GetPhysicsLinearVelocity (Variables|Default|GetObject) "None"))
  (if (> (Math|Vector|VectorLength _returnvalue) _maxvelocity)
    (Physics|SetPhysicsLinearVelocity (Variables|Default|GetObject) (Math|Vector|VectorClampSizeMax _returnvalue _maxvelocity) false "None")))

(fn Ungrab
  (bind _object (Variables|Default|GetObject))
  (Transformation|DetachFromComponent _object "KeepWorld" "KeepWorld" "KeepRelative" true)
  (Physics|SetSimulatePhysics _object true)
  (Variables|Default|SetGrab? false))

(fn Grab
  (Transformation|AttachComponentToComponent (Variables|/Game/Character/BP_FirstPersonCharacter.BP_FirstPersonCharacter_C|GetGrabLocation (Variables|Default|GetAs%20BP%20First%20Person%20Character)) "None" "KeepWorld" "KeepWorld" "KeepRelative" true)
  (Variables|Default|SetGrab? true))

(fn InterpolateGrabbing
  (params (Delta :type Float%20%28double-precision%29) (Speed :type Float%20%28double-precision%29))
  (bind _object (Variables|Default|GetObject))
  (Transformation|SetWorldTransform _object (Math|Transform|Lerp(Transform) (Transformation|GetWorldTransform _object) (Transformation|GetWorldTransform (Variables|/Game/Character/BP_FirstPersonCharacter.BP_FirstPersonCharacter_C|GetGrabLocation (Variables|Default|GetAs%20BP%20First%20Person%20Character))) (* Delta Speed)) false false))